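; BP_PopupActor is a trigger volume that shows a text popup when the player character enters its box.
; On overlap it finds the existing UI_Popup widget, copies in its own Text, makes it visible, then hides it after a fixed delay.
; A HasShown flag gates the popup, but nothing in these graphs sets it.
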(event `self.Box.OnComponentBeginOverlap`
  (params (OverlappedComponent :type "PrimitiveComponent Object Reference") (OtherActor :type "Actor Object Reference") (OtherComp :type "PrimitiveComponent Object Reference") (OtherBodyIndex :type Integer) (bFromSweep :type Boolean) (SweepResult :type "HitResult Structure (by ref)"))
  (if (not (`self.HasShown`))
    (cast `PlayerCharacter` OtherActor)
    (bind _foundwidgets (`WidgetBlueprintLibrary.GetAllWidgetsOfClass` "/Game/BP/UI_Popup.UI_Popup_C" false))
    (bind _output (`|GetArrayItem` _foundwidgets))
    (`/Engine/EditorBlueprintResources/StandardMacros.IsValid` _output
      (:`Is Valid`
        (set `/Game/BP/UI_Popup.Text` (`self.Text`) _output)
        (`Widget.SetVisibility` _output "Visible")
        (`KismetSystemLibrary.Delay` 5.0)
        (`Widget.SetVisibility` _output "Hidden")))))

(fn `UserConstructionScript`)