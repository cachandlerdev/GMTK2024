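; Player character Blueprint that adds feedback for movement events (crouch, slide, sprint, dash, mantle, jump) and creates the HUD and pause menu.
; A reversible timeline lerps capsule half-height for crouching, with a slide sound when crouch starts above jog speed on the ground.
; Sprinting shows speed lines and recursively replays a camera shake while moving.
; Dash and mantle trigger their own shakes, while dash and ground or air jumps play sounds.
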(event `self.ReceiveBeginPlay`
  (bind _capsulehalfheight (`CapsuleComponent.CapsuleHalfHeight` (`self.CapsuleComponent`)))
  ;[1 1 1] Comment
  (set `self.InitialHeight` _capsulehalfheight)
  (set `self.CrouchHeight` (/ _capsulehalfheight 2.0))
  (bind _returnvalue (`|CreateWidget` "/Game/BP/UI/UI_Hud.UI_Hud_C" (`GameplayStatics.GetPlayerController` 0)))
  (`UserWidget.AddToViewport` _returnvalue 0)
  (set `self.HudMenu` _returnvalue))

(event `self.StartCrouch`
  ;[1 1 1] Crouch
  (`self.SlideSoundEffect`)
  (bind (_direction _value) (`Timeline|CrouchTimeline` :!label _label)
    (:`Update`
      (`CapsuleComponent.SetCapsuleHalfHeight` (`self.CapsuleComponent`) (`KismetMathLibrary.Lerp` (`self.InitialHeight`) (`self.CrouchHeight`) _value) true))))

(event `self.EndCrouch`
  ;[1 1 1] Crouch
  (set `self.IsSliding` false)
  (goto _label :!via `Reverse`))

(event `self.DoWhileSprinting`
  ;[1 1 1] Comment
  (if (not (`self.bHasStartedSprinting`))
    (set `self.bHasStartedSprinting` true)
    (`SceneComponent.SetVisibility` (`self.SpeedLines`) true false)
    (`self.KeepShakingCamera`)))

(event `KeepShakingCamera`
  ;[1 1 1] Comment
  (if (and (> (`KismetMathLibrary.VSize` (`self.GetVelocity`)) 10.0) (not (`self.bIsShaking`)))
    (set `self.bIsShaking` true)
    (bind _returnvalue (`LegacyCameraShake.StartLegacyCameraShake` (`GameplayStatics.GetPlayerCameraManager` 0) "/Game/Blueprints/Player/BP_CameraShake.BP_CameraShake_C"))
    (bind _returnvalue_2 (message `AnimationDataModel.GetPlayLength` _returnvalue))
    (`KismetSystemLibrary.Delay` _returnvalue_2)
    (set `self.bIsShaking` false)
    (`self.KeepShakingCamera`)))

(event `self.DoWhenSprintingOver`
  ;[1 1 1] Comment
  (set `self.bIsShaking` false)
  (set `self.bHasStartedSprinting` false)
  (`SceneComponent.SetVisibility` (`self.SpeedLines`) false false))

(event `self.OnDash`
  ;[1 1 1] Comment
  (`LegacyCameraShake.StartLegacyCameraShake` (`GameplayStatics.GetPlayerCameraManager` 0) "/Game/Blueprints/Player/BP_DashShake.BP_DashShake_C")
  (`GameplayStatics.PlaySoundAtLocation` (`self.DashSound`) (`self.K2_GetActorLocation`) (struct) 1.0 1.0 0.0 null null null null))

(event `self.OnMantle`
  ;[1 1 1] Comment
  (`LegacyCameraShake.StartLegacyCameraShake` (`GameplayStatics.GetPlayerCameraManager` 0) "/Game/Blueprints/Player/BP_MantleShake.BP_MantleShake_C"))

(event `self.OnJump`
  (params (bIsAirJump :type Boolean))
  ;[1 1 1] Comment
  (if bIsAirJump
    (`GameplayStatics.PlaySoundAtLocation` (`self.AirJump`) (`self.K2_GetActorLocation`) (struct) 1.0 1.0 0.0 null null null null)
    (else
      (`GameplayStatics.PlaySoundAtLocation` (`self.RegularJump`) (`self.K2_GetActorLocation`) (struct) 1.0 1.0 0.0 null null null null))))

(event `EnhancedInput|/Game/Input/Actions/IA_MenuAction`
  (params (ActionValue :type Boolean) (ElapsedSeconds :type "Float (double-precision)") (TriggeredSeconds :type "Float (double-precision)") (InputAction :type "InputAction Object Reference" :default "/Game/Input/Actions/IA_MenuAction.IA_MenuAction"))
  ;[1 1 1] Comment
  (:`Triggered`
    (bind _returnvalue (`|CreateWidget` "/Game/BP/UI/UI_PauseMenu.UI_PauseMenu_C" (`GameplayStatics.GetPlayerController` 0)))
    (bind _output_get (set `self.PauseMenu` _returnvalue))
    (`UserWidget.AddToViewport` _output_get 0)))

(fn `SlideSoundEffect`
  (if (not (`self.IsSliding`))
    (if (and (> (`KismetMathLibrary.VSize` (`MovementComponent.Velocity` (`self.CharacterMovement`))) (`self.jogSpeed`)) (not (`NavMovementComponent.IsFalling` (`self.CharacterMovement`))))
      (`GameplayStatics.PlaySoundAtLocation` (`self.SlideSound`) (`self.K2_GetActorLocation`) (struct) 1.0 1.0 0.0 null null null null)
      (set `self.IsSliding` true))))

(fn `UserConstructionScript`)