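; Game mode Blueprint for a ship-construction game, linking shift timer, quota and order tickets to their displays.
; On BeginPlay it records the ship spawn location, advances the game instance's music track and caches the player's HUD.
; A self-calling UpdateTimer event with a short delay keeps build time current on the HUD.
; Other events refresh the quota and ticket boards, and shift end shows a report card widget.
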(event `self.ReceiveBeginPlay`
  ;[1 1 1] Begin play
  (bind _returnvalue (`GameplayStatics.GetActorOfClass` "/Game/BP/BP_ShipSpawnLocation.BP_ShipSpawnLocation_C"))
  (`/Engine/EditorBlueprintResources/StandardMacros.IsValid` _returnvalue
    (:`Is Valid`
      (set `self.shipConstructionLocation` (`self.K2_GetActorLocation` _returnvalue)))
    (:`Is Not Valid`
      _))
  (bind _asbp_my_game_instance (cast `/Game/BP/BP_MyGameInstance` (`GameplayStatics.GetGameInstance`))
    (:`then`
      (`MyGameInstance.GoToNextMusicTrack` _asbp_my_game_instance)
      (`KismetSystemLibrary.Delay` 0.01))
    (:`CastFailed`
      _))
  (bind _asbp_player_character (cast `/Game/BP/BP_PlayerCharacter` (`GameplayStatics.GetPlayerCharacter` 0)))
  (set `self.PlayerHud` (`/Game/BP/BP_PlayerCharacter.HudMenu` _asbp_player_character))
  (`self.UpdateTimer`))

(event `self.PartAddedBP`
  (params (Ticket :type "TicketActor Object Reference"))
  ;[1 1 1] Part added
  (bind _asticket_board_actor_bp (cast `/Game/Blueprints/Env/TicketBoardActorBP` (`TicketActor.TicketBoard` Ticket)))
  (`/Game/Blueprints/Env/TicketBoardActorBP.UpdateDisplay` _asticket_board_actor_bp (`TicketActor.progressOrder` Ticket) (`TicketActor.order` Ticket)))

(event `self.AddOrderBP`
  ;[1 1 1] Add order
)

(event `UpdateTimer`
  (`/Engine/EditorBlueprintResources/StandardMacros.IsValid` (`self.PlayerHud`)
    (:`Is Valid`
      (`/Game/BP/UI/UI_Hud.UpdateTimer` (`self.PlayerHud`) (`self.buildTime`))
      (`KismetSystemLibrary.Delay` 0.01)
      (`self.UpdateTimer`))))

(event `self.UpdateQuotaBP`
  (bind _playerhud (`self.PlayerHud`))
  (`/Engine/EditorBlueprintResources/StandardMacros.IsValid` _playerhud
    (:`Is Valid`
      (`/Game/BP/UI/UI_Hud.UpdateQuota` _playerhud (`self.shiftQuota`)))))

(event `self.OnShiftEnd`
  (bind _returnvalue (`|CreateWidget` "/Game/BP/UI/UI_ReportCard.UI_ReportCard_C" (`GameplayStatics.GetPlayerController` 0) (`OrderDataSheet.reports` (`self.orderSheet`))))
  (`UserWidget.AddToViewport` _returnvalue 0))

(fn `Init`)

(fn `UserConstructionScript`)