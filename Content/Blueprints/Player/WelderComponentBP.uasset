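; Welder component, filed under Player, that handles the sound for welding start and end events.
; OnStartWeld spawns WelderSound at the owner's location and stores the reference, and OnEndWeld stops that stored sound if it is still valid.
; The IsPlayingSound flag does not prevent repeat spawns, and the start event sets it true only when it is already true.
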(event `self.OnStartWeld`
  (if (`self.IsPlayingSound`)
    (set `self.IsPlayingSound` true))
  (bind _returnvalue (`GameplayStatics.SpawnSoundAtLocation` (`self.WelderSound`) (`Actor.K2_GetActorLocation` (`self.GetOwner`)) (struct) 1.0 1.0 0.0 null null))
  (set `self.WelderSoundInWorld` _returnvalue))

(event `self.OnEndWeld`
  (bind _weldersoundinworld (`self.WelderSoundInWorld`))
  (set `self.IsPlayingSound` false)
  (`/Engine/EditorBlueprintResources/StandardMacros.IsValid` _weldersoundinworld
    (:`Is Valid`
      (`AudioComponent.StopDelayed` _weldersoundinworld 0.0))))