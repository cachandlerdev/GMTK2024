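; Player character Blueprint that adds sprint feedback and smooth crouching.
; BeginPlay caches the camera FOV and capsule height, then Tick widens the FOV up to a cap while speed exceeds jog speed and eases it back otherwise.
; Sprint events start a camera shake and toggle speed lines.
; Crouch events play or reverse a timeline that lerps the capsule between full and half height.
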(event `self.ReceiveBeginPlay`
  (bind _capsulehalfheight (`CapsuleComponent.CapsuleHalfHeight` (`self.CapsuleComponent`)))
  (bind _fieldofview (`CameraComponent.FieldOfView` (`self.Camera`)))
  ;[1 1 1] Comment
  (set `self.InitialFov` _fieldofview)
  (set `self.MaxFov` (+ _fieldofview (`self.SprintFovIncrease`)))
  (set `self.InitialHeight` _capsulehalfheight)
  (set `self.CrouchHeight` (/ _capsulehalfheight 2.0))
  (set `self.CameraLocation` (`SceneComponent.RelativeLocation` (`self.Camera`))))

(event `self.ReceiveTick`
  (params (DeltaSeconds :type "Float (single-precision)"))
  (bind _camera (`self.Camera`))
  (bind _fieldofview (`CameraComponent.FieldOfView` _camera))
  (set `self.DeltaTime` DeltaSeconds)
  (if (> (`KismetMathLibrary.VSize` (`self.GetVelocity`)) (+ (`self.jogSpeed`) 10.0))
    (`CameraComponent.SetFieldOfView` _camera (`KismetMathLibrary.FClamp` (`KismetMathLibrary.Lerp` _fieldofview (+ _fieldofview (`self.SprintFovIncrease`)) (`self.DeltaTime`)) 0.0 (`self.MaxFov`)))
    (else
      (`CameraComponent.SetFieldOfView` (`self.Camera`) (`KismetMathLibrary.Lerp` (`CameraComponent.FieldOfView` (`self.Camera`)) (`self.InitialFov`) (* (`self.DeltaTime`) 5.0))))))

(event `self.DoWhileSprinting`
  ;[1 1 1] Comment
  (`LegacyCameraShake.StartLegacyCameraShake` (`GameplayStatics.GetPlayerCameraManager` 0) "/Game/Blueprints/Player/BP_CameraShake.BP_CameraShake_C")
  (`SceneComponent.SetVisibility` (`self.SpeedLines`) true false))

(event `self.StartCrouch`
  ;[1 1 1] Crouch
  (bind (_direction _value) (`Timeline|CrouchTimeline` :!label _label)
    (:`Update`
      (`CapsuleComponent.SetCapsuleHalfHeight` (`self.CapsuleComponent`) (`KismetMathLibrary.Lerp` (`self.InitialHeight`) (`self.CrouchHeight`) _value) true))))

(event `self.EndCrouch`
  ;[1 1 1] Crouch
  (goto _label :!via `Reverse`))

(event `self.DoWhenSprintingOver`
  ;[1 1 1] Comment
  (`SceneComponent.SetVisibility` (`self.SpeedLines`) false false))

(fn `UserConstructionScript`)